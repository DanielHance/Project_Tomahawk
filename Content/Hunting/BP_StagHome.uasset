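; Stag home actor that populates the hunting world by spawning BP_Stag at the location of its static mesh.
; On BeginPlay it spawns one immediately, then another every ten seconds through a Delay loop until Population reaches MaxPopulation.
; Each stag receives the home location and randomized energy, hunger and health stats, with current and max values rolled in separate calls.
; Population only counts up, so dead stags are not replaced.
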(event `self.ReceiveBeginPlay`
  (bind _returnvalue (`KismetMathLibrary.RandomIntegerInRange` 100 200))
  (bind _returnvalue_2 (`KismetMathLibrary.RandomIntegerInRange` 150 300))
  (bind _returnvalue_3 (`KismetMathLibrary.RandomIntegerInRange` 50 150))
  (bind _output_get (set `self.Home Location` (`SceneComponent.K2_GetComponentLocation` (`self.StaticMesh`))))
  (set `self.Population` 0)
  (`|SpawnActorFromClass` "/Game/Hunting/BP_Stag.BP_Stag_C" (`KismetMathLibrary.Conv_VectorToTransform` _output_get) "Undefined" "OverrideRootScale" null _returnvalue_2 5 _returnvalue_2 5 _returnvalue 5 _returnvalue 25 _returnvalue_3 2 _returnvalue_3 3 _output_get null :!label _label)
  (bind _output_get_2 (set `self.Population` (+ (`self.Population`) 1)))
  (`KismetSystemLibrary.Delay` 10.0)
  (if (< _output_get_2 (`self.MaxPopulation`))
    (goto _label)))

(fn `UserConstructionScript`)
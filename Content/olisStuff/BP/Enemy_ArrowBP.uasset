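; Enemy arrow actor that can hurt the player when its hitbox touches the third-person character.
; The first such overlap passes a DoOnce and rolls a one-in-three chance to subtract a fixed amount from PlayerHealth directly.
; A successful roll also prints a debug string, plays a damage sound at world origin and destroys the arrow.
; A failed roll leaves the arrow in place, unable to damage again because the DoOnce never resets.
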(event `self.Arrow_Hitbox.OnComponentBeginOverlap`
  (params (OverlappedComponent :type "PrimitiveComponent Object Reference") (OtherActor :type "Actor Object Reference") (OtherComp :type "PrimitiveComponent Object Reference") (OtherBodyIndex :type Integer) (bFromSweep :type Boolean) (SweepResult :type "HitResult Structure (by ref)"))
  (bind _asbp_third_person_character (cast `/Game/ThirdPerson/Blueprints/BP_ThirdPersonCharacter` OtherActor))
  (`/Engine/EditorBlueprintResources/StandardMacros.DoOnce` false
    (:`Completed`
      (if (== (`KismetMathLibrary.RandomIntegerInRange` 1 3) 1)
        (set `/Game/ThirdPerson/Blueprints/BP_ThirdPersonCharacter.playerHealth` (- (`/Game/ThirdPerson/Blueprints/BP_ThirdPersonCharacter.playerHealth` _asbp_third_person_character) 20.0) _asbp_third_person_character)
        (`KismetSystemLibrary.PrintString` "+++++++++++++++++++++++++++++++++++++++++++++++++++++++++++++++")
        (`GameplayStatics.PlaySoundAtLocation` "/Game/olisStuff/SFX/DamageSound.DamageSound" (0.0 0.0 0.0) (struct) 1.0 1.0 0.0 null null null null)
        (`self.K2_DestroyActor`)))))

(fn `UserConstructionScript`)
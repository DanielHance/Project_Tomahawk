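; Homing arrow projectile that seeks actors tagged "Homing" and damages enemies on contact.
; From BeginPlay it re-runs LockOn on a short repeating delay, feeding the chosen target's scene component into ProjectileMovement's homing.
; Target search keeps the nearest tagged actor, comparing against a stored closest distance that is never reset between searches.
; Sphere overlap with an Enemy calls DealDamageHoming and destroys the arrow.
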(event `Lock On`
  (bind _projectilemovement (`self.ProjectileMovement`))
  (bind _homingtarget (`self.findhomingtarget`))
  (set `ProjectileMovementComponent.HomingTargetComponent` _homingtarget _projectilemovement)
  (set `ProjectileMovementComponent.bIsHomingProjectile` true _projectilemovement))

(event `self.ReceiveBeginPlay`
  (`self.Lock On` :!label _label)
  (`KismetSystemLibrary.Delay` 0.2)
  (goto _label))

(event `self.Sphere1.OnComponentBeginOverlap`
  (params (OverlappedComponent :type "PrimitiveComponent Object Reference") (OtherActor :type "Actor Object Reference") (OtherComp :type "PrimitiveComponent Object Reference") (OtherBodyIndex :type Integer) (bFromSweep :type Boolean) (SweepResult :type "HitResult Structure (by ref)"))
  (bind _asenemy (cast `/Game/olisStuff/BP/Enemy` OtherActor))
  (`/Game/olisStuff/BP/Enemy.DealDamage_Homing` _asenemy)
  (`self.K2_DestroyActor`))

(fn `findhomingtarget`
  (returns (homingTarget :type "SceneComponent Object Reference"))
  (bind _outactors (`GameplayStatics.GetAllActorsOfClassWithTag` "/Script/Engine.Actor" "Homing"))
  (for _array_element _outactors
    (bind _returnvalue (`KismetMathLibrary.VSize` (- (`self.K2_GetActorLocation` _array_element) (`self.K2_GetActorLocation`))))
    (if (< _returnvalue (`self.closestDistance`))
      (set `self.closestDistance` _returnvalue)
      (set `self.currentHomingTarget` _array_element)))
  (return (`self.GetComponentByClass` (`self.currentHomingTarget`) "/Script/Engine.SceneComponent")))

(fn `UserConstructionScript`)
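; An enemy spawner actor that spawns escalating batches of enemies at its own transform.
; On BeginPlay it binds its spawn event to the respawn-enemy dispatcher on BP_ThirdPersonGameMode, so the game mode drives when batches appear.
; Each call spawns the current count, ignoring collisions, then raises an increment and adds it to the count, so batch growth accelerates with every call.
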(event `self.ReceiveBeginPlay`
  (bind _asbp_third_person_game_mode (cast `/Game/ThirdPerson/Blueprints/BP_ThirdPersonGameMode` (`GameplayStatics.GetGameMode`)))
  (add `/Game/ThirdPerson/Blueprints/BP_ThirdPersonGameMode.RespawnEnemy` _asbp_third_person_game_mode (delegate `spawnEnemy`)))

(event `spawnEnemy`
  (for _ (range (`self.enemySpawned`))
    (`|SpawnActorFromClass` "/Game/olisStuff/BP/Enemy.Enemy_C" (`self.GetTransform`) "AlwaysSpawn" "OverrideRootScale" null null))
  (`/Engine/EditorBlueprintResources/StandardMacros.IncrementInt` (`self.spawnIncrement`)
    (:`  `
      (set `self.enemySpawned` (+ (`self.enemySpawned`) (`self.spawnIncrement`))))))

(fn `UserConstructionScript`)
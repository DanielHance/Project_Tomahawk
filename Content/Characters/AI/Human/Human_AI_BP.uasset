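; Human enemy AI character that switches between knife and bow combat and takes damage from player weapons.
; Blackboard CombatState drives weapon draw/stow montages, which set walk speed, while ResetCombat stows and returns both states to default.
; ShotBow spawns enemy arrows from a spawn component.
; Capsule overlaps set damage by projectile or knife type, then subtract health through DoOnce gates; death only prints a message.
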(event `Weapon Check`
  ;[1 1 1] Changes weapon when combat states change
  (`KismetSystemLibrary.PrintString` "Weaon check")
  (switch `/Game/Characters/AI/Human/Enums/Human_CombatState_Enum` (cast `/Game/Characters/AI/Human/Enums/Human_CombatState_Enum` (`BlackboardComponent.GetValueAsEnum` (`AIBlueprintHelperLibrary.GetBlackboard` null) "CombatState"))
    (:`NewEnumerator1`
      (if (`self.RangeCombat`)
        (`self.Stow Bow`)
        (`KismetSystemLibrary.Delay` 1.0))
      (`self.Draw Knife`)
      (set `self.MeleeCombat` true))
    (:`NewEnumerator2`
      (if (`self.MeleeCombat`)
        (`self.Stow Knife`)
        (`KismetSystemLibrary.Delay` 1.0))
      (`self.Draw Bow`)
      (set `self.RangeCombat` true))))

(event `Reset Combat`
  (bind _returnvalue (`AIBlueprintHelperLibrary.GetBlackboard` null))
  ;[1 1 1] Puts away weapon after combat (also chanegs base and combat states to defult)
  (switch `/Game/Characters/AI/Human/Enums/Human_CombatState_Enum` (cast `/Game/Characters/AI/Human/Enums/Human_CombatState_Enum` (`BlackboardComponent.GetValueAsEnum` (`AIBlueprintHelperLibrary.GetBlackboard` null) "CombatState"))
    (:`NewEnumerator1`
      (`self.Stow Knife`))
    (:`NewEnumerator2`
      (`self.Stow Bow`)))
  (set `self.RangeCombat` false)
  (set `self.MeleeCombat` false)
  (`KismetSystemLibrary.Delay` 1.0)
  (`BlackboardComponent.SetValueAsEnum` _returnvalue "CombatState" 0)
  (`BlackboardComponent.SetValueAsEnum` _returnvalue "BaseState" 0))

(event `Draw Knife`
  ;[1 1 1] Plays draw and stow animations
  (`|PlayMontage` null "/Game/CloseCombatAnimSet/Animations/Montages/Draw_Knife_FILLER.Draw_Knife_FILLER"
    (:`then`
      (set `CharacterMovementComponent.MaxWalkSpeed` 250.0 (`self.CharacterMovement`) :!label _label)
      (`KismetSystemLibrary.PrintString` "animation played"))))

(event `Shot Bow`
  (bind _arrowprojectilespawn (`self.ArrowProjectileSpawn`))
  (`KismetSystemLibrary.PrintString` "Shot Arrow")
  (`|SpawnActorFromClass` "/Game/olisStuff/BP/Enemy_ArrowBP.Enemy_ArrowBP_C" (`KismetMathLibrary.MakeTransform` (`SceneComponent.K2_GetComponentLocation` _arrowprojectilespawn) (`KismetMathLibrary.MakeRotFromZ` (`SceneComponent.GetForwardVector` _arrowprojectilespawn)) (2.0 2.0 2.0)) "Undefined" "OverrideRootScale" null null))

(event `Draw Bow`
  ;[1 1 1] Plays draw and stow animations
  (`KismetSystemLibrary.PrintString` "Draw Bow")
  (`|PlayMontage` null "/Game/CloseCombatAnimSet/Animations/Montages/Draw_Bow_FILLER.Draw_Bow_FILLER"
    (:`then`
      (goto _label))))

(event `Stow Knife`
  ;[1 1 1] Plays draw and stow animations
  (`|PlayMontage` null "/Game/CloseCombatAnimSet/Animations/Montages/Stow_Knife_FILLER.Stow_Knife_FILLER"
    (:`then`
      (set `CharacterMovementComponent.MaxWalkSpeed` 175.0 (`self.CharacterMovement`) :!label _label_2))))

(event `Stow Bow`
  ;[1 1 1] Plays draw and stow animations
  (`|PlayMontage` null "/Game/CloseCombatAnimSet/Animations/Montages/Stow_Bow_FILLER.Stow_Bow_FILLER"
    (:`then`
      (goto _label_2))))

(event `self.ReceiveBeginPlay`
  (set `self.enemyAI_Ref` self))

(event `self.CapsuleComponent.OnComponentBeginOverlap`
  (params (OverlappedComponent :type "PrimitiveComponent Object Reference") (OtherActor :type "Actor Object Reference") (OtherComp :type "PrimitiveComponent Object Reference") (OtherBodyIndex :type Integer) (bFromSweep :type Boolean) (SweepResult :type "HitResult Structure (by ref)"))
  ;[1 1 1] Damage vs AI test
  (cast `/Game/olisStuff/BP/ArrowBP` OtherActor
    (:`then`
      (set `self.DamageNo` 50.0))
    (:`CastFailed`
      (cast `/Game/olisStuff/BP/KnifeBP` OtherActor
        (:`then`
          (set `self.DamageNo` 34.0))
        (:`CastFailed`
          (cast `/Game/olisStuff/BP/QuickShotArrowBP` OtherActor
            (:`then`
              (set `self.DamageNo` 50.0))
            (:`CastFailed`
              (bind _astomohawk_bp (cast `/Game/olisStuff/BP/TomohawkBP` OtherActor))
              (`self.K2_DestroyActor` _astomohawk_bp)
              (set `self.DamageNo` 100.0)))))))
  (`/Engine/EditorBlueprintResources/StandardMacros.DoOnce` false
    (:`Completed`
      (`self.DealDamage`))))

(event `DealDamage`
  ;[1 1 1] Damage vs AI test
  (`/Engine/EditorBlueprintResources/StandardMacros.DoOnce` false :!label _label_3
    (:`Completed`
      (bind _output_get (set `self.maxHealth_AI` (- (`self.maxHealth_AI`) (`self.DamageNo`))))
      (if (<= _output_get 0.0)
        (`KismetSystemLibrary.PrintString` "AI HUMAN DEAD!!!!!")
        (else
          (goto _label_3 :!via `Reset`))))))

(fn `UserConstructionScript`)
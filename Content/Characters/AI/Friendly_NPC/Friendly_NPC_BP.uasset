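; Friendly NPC that wanders at random by day with a pet bird or wolf and heads home at night.
; Tick sets the return-home flag from the Day variable and destroys the NPC when it is far from the player.
; A randomly delayed action loop picks wander or go home via AI MoveTo, re-entering after each successful move.
; Wandering spawns an owner-linked pet if none exists; arriving home sets Sleep and destroys it.
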(event `self.ReceiveTick`
  (params (DeltaSeconds :type "Float (single-precision)"))
  ;[1 1 1] De-spawning
  (if (> (`KismetMathLibrary.Vector_Distance` (`self.K2_GetActorLocation` (`GameplayStatics.GetPlayerCharacter` 0)) (`self.K2_GetActorLocation`)) 15000.0)
    (`self.K2_DestroyActor`)
    (else
      ;[1 1 1] Check Time
      (if (`self.Day?`)
        (set `self.Return Home` false)
        (else
          (set `self.Return Home` true))))))

(event `Move Rand Loc`
  ;[1 1 1] Random Move
  (set `self.Sleep` false)
  (`|AIMoveTo` self (`NavigationSystemV1.K2_GetRandomReachablePointInRadius` (`self.K2_GetActorLocation`) 1000.0 null null) null
    (:`OnSuccess`
      (`self.Pick Action`))))

(event `Move Home`
  ;[1 1 1] Return Home
  (`|AIMoveTo` self (0.0 0.0 0.0) (`self.Home`)
    (:`OnSuccess`
      (set `self.Sleep` true)
      (`self.Pick Action`)
      (`KismetSystemLibrary.Delay` 0.5)
      (bind _pet_ref (`self.Pet Ref`)
        (:`then`
          (`self.K2_DestroyActor` _pet_ref))
        (:`else`)))))

(event `self.ReceiveBeginPlay`
  (bind _returnvalue (`KismetMathLibrary.Conv_VectorToTransform` (`self.K2_GetActorLocation`)))
  ;[1 1 1] Select Move
  (`KismetSystemLibrary.Delay` (`KismetMathLibrary.RandomFloatInRange` 0.1 5.0) :!label _label)
  (if (`self.Return Home`)
    (`self.Move Home`)
    (else
      (`self.Move Rand Loc`)
      (`self.Pet Ref`
        (:`then`)
        (:`else`
          (if (`self.Bird`)
            (bind _returnvalue_2 (`|SpawnActorFromClass` "/Game/Characters/AI/Friendly_NPC/Friendly_NPC_Bird_BP.Friendly_NPC_Bird_BP_C" _returnvalue "AdjustIfPossibleButAlwaysSpawn" "OverrideRootScale" null null))
            (set `self.Pet Ref` _returnvalue_2)
            (set `/Game/Characters/AI/Friendly_NPC/Friendly_NPC_Bird_BP.Owner Ref` self _returnvalue_2)
            (else
              (bind _returnvalue_3 (`|SpawnActorFromClass` "/Game/Characters/AI/Friendly_NPC/Friendly_NPC_Wolf_BP.Friendly_NPC_Wolf_BP_C" _returnvalue "AdjustIfPossibleButAlwaysSpawn" "OverrideRootScale" null null))
              (set `self.Pet Ref` _returnvalue_3)
              (set `/Game/Characters/AI/Friendly_NPC/Friendly_NPC_Wolf_BP.Owner Ref` self _returnvalue_3))))))))

(event `Pick Action`
  ;[1 1 1] Select Move
  (goto _label))

(fn `UserConstructionScript`)
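; Player bird AI character, a sprite animal tied to an owning player that can be given a target and told to attack.
; On spawn it stores the owner as Player and passes a multiple of its DamageStrength to that player's SetHealthMessage; despawn destroys the actor.
; SetTarget stores the target, and both it and Attack switch the Bird State blackboard enum, with debug prints.
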(event `/Game/Characters/AI/SpriteAnimalInterface.SpawnSpriteAnimal`
  (params (Owner :type "Actor Object Reference"))
  (set `self.Player` Owner)
  (`KismetSystemLibrary.PrintString` (`KismetStringLibrary.Conv_VectorToString` (`self.K2_GetActorLocation`)))
  (message `/Game/Characters/AI/SpriteAnimalInterface.SetHealth` (`self.Player`) (* (`self.DamageStrength`) 3.0)))

(event `/Game/Characters/AI/SpriteAnimalInterface.DespawnSpriteAnimal`
  (`self.K2_DestroyActor`))

(event `/Game/Characters/AI/SpriteAnimalInterface.SetTarget`
  (params (Target :type "Actor Object Reference"))
  (set `self.Target` Target)
  (`BlackboardComponent.SetValueAsEnum` (`AIBlueprintHelperLibrary.GetBlackboard` null) "Bird State" 1)
  (`KismetSystemLibrary.PrintString` "Target Set"))

(event `Attack`
  (`KismetSystemLibrary.PrintString` "Attack")
  (`BlackboardComponent.SetValueAsEnum` (`AIBlueprintHelperLibrary.GetBlackboard` null) "Bird State" 2))

(fn `UserConstructionScript`)
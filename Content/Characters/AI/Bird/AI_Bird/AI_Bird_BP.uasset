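; Bird AI Blueprint that switches the bird's behavior through a "Bird State" enum key on its Blackboard.
; SetTarget stores the given target in a variable and sets state 1, while Attack prints a debug string and sets state 2.
; DespawnSpriteAnimal destroys the actor, and the construction script is empty.
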(event `/Game/Characters/AI/SpriteAnimalInterface.DespawnSpriteAnimal`
  (`self.K2_DestroyActor`))

(event `/Game/Characters/AI/SpriteAnimalInterface.SetTarget`
  (params (Target :type "Actor Object Reference"))
  (set `self.Target` Target)
  (`BlackboardComponent.SetValueAsEnum` (`AIBlueprintHelperLibrary.GetBlackboard` null) "Bird State" 1))

(event `Attack`
  (`KismetSystemLibrary.PrintString` "Attack")
  (`BlackboardComponent.SetValueAsEnum` (`AIBlueprintHelperLibrary.GetBlackboard` null) "Bird State" 2))

(fn `UserConstructionScript`)
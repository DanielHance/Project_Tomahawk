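; Player-owned wolf "sprite animal" with spawn, despawn, targeting and attack events.
; On spawn it stores its owner as Player and sends that player a health message of half DamageStrength.
; SetTarget stores the target and sets the blackboard enum "Bird State" to 1, a key named for a bird despite the wolf.
; Despawn destroys the actor, while Attack is a stub that only prints.
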(event `/Game/Characters/AI/SpriteAnimalInterface.SpawnSpriteAnimal`
  (params (Owner :type "Actor Object Reference"))
  (set `self.Player` Owner)
  (`KismetSystemLibrary.PrintString` (`KismetStringLibrary.Conv_VectorToString` (`self.K2_GetActorLocation`)))
  (message `/Game/Characters/AI/SpriteAnimalInterface.SetHealth` (`self.Player`) (* (`self.DamageStrength`) 0.5))
  (`KismetSystemLibrary.PrintString` "WOLF"))

(event `/Game/Characters/AI/SpriteAnimalInterface.DespawnSpriteAnimal`
  (`self.K2_DestroyActor`))

(event `/Game/Characters/AI/SpriteAnimalInterface.SetTarget`
  (params (Target :type "Actor Object Reference"))
  (set `self.Target` Target)
  (`BlackboardComponent.SetValueAsEnum` (`AIBlueprintHelperLibrary.GetBlackboard` null) "Bird State" 1))

(event `Attack`
  (`KismetSystemLibrary.PrintString` "Attack"))

(fn `UserConstructionScript`)
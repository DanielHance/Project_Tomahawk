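; BP_FirePlace is a placeable fireplace prop with selectable mesh variant and fire type, configured in the construction script.
; The clamped MeshVariant index picks the static mesh from the Meshes array.
; FireType looks up the particle template and point light intensity in maps, while one enum value instead destroys both the fire and light components.
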(fn `UserConstructionScript`
  (bind (_value _returnvalue) (`BlueprintMapLibrary.Map_Find` (`self.Particles`) (`self.FireType`)))
  (set `self.MeshVariant` (`KismetMathLibrary.Max` (`KismetMathLibrary.Min` (`self.MeshVariant`) (- (`KismetArrayLibrary.Array_Length` (`self.Meshes`)) 1))))
  (`StaticMeshComponent.SetStaticMesh` (`self.StaticMeshComponent`) (`|GetArrayItem` (`self.Meshes`) (`self.MeshVariant`)))
  (if (`|EnumInequality` (`self.FireType`) "NewEnumerator3")
    (if _returnvalue
      (`ParticleSystemComponent.SetTemplate` (`self.Fire`) _value)
      (`LightComponent.SetIntensity` (`self.PointLight`) (`BlueprintMapLibrary.Map_Find` (`self.LightIntensity`) (`self.FireType`))))
    (else
      (`ActorComponent.K2_DestroyComponent` (`self.Fire`))
      (`ActorComponent.K2_DestroyComponent` (`self.PointLight`)))))